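; Boss_BP is a ghost boss that shows at full opacity when GlassesOn is set and otherwise flickers in and out.
; The construction script creates a dynamic material instance, whose "Opacidad" parameter Tick sets to solid or to a time-driven sine wave.
; DieGhosts flags it dead, swaps to a wormhole material, stops the Ghosts_AIControlller brain logic and sets a short lifespan for removal.
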(event `self.ReceiveTick`
  (params (DeltaSeconds :type "Float (single-precision)"))
  (if (`self.GlassesOn`)
    (`MaterialInstanceDynamic.SetScalarParameterValue` (`self.GhostsMaterial`) "Opacidad" 1.0)
    (else
      (set `self.Time` (+ DeltaSeconds (`self.Time`)))
      (`MaterialInstanceDynamic.SetScalarParameterValue` (`self.GhostsMaterial`) "Opacidad" (* 0.8 (`KismetMathLibrary.Sin` (/ (`self.Time`) 0.3)))))))

(fn `DieGhosts`
  (set `self.Dead` true)
  (`PrimitiveComponent.SetMaterial` (`self.StaticMesh`) 0 "/Game/Project/WormHole_Inst.WormHole_Inst")
  (`self.SetLifeSpan` 1.0)
  (`BrainComponent.StopLogic` (`AIController.BrainComponent` (cast `/Game/Project/Ghosts_AIControlller` (`AIBlueprintHelperLibrary.GetAIController` self) :!pure true)) ""))

(fn `UserConstructionScript`
  (bind _returnvalue (`PrimitiveComponent.CreateDynamicMaterialInstance` (`self.StaticMesh`) 0 "/Game/Project/GhostMaterial_instance.GhostMaterial_instance" "None"))
  (set `self.GhostsMaterial` _returnvalue))