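; GameInstance Blueprint that provides save-game handling, with Save as its only implemented event.
; Save creates a fresh SaveGame_BP, copies score, life, power and transform from player 0's ThirdPersonCharacter, and writes it to a fixed slot.
; Restart and Load events are declared but empty.
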(event `Restart`)

(event `Save`
  (bind _asthird_person_character (cast `/Game/ThirdPersonBP/Blueprints/ThirdPersonCharacter` (`GameplayStatics.GetPlayerCharacter` 0) :!pure true))
  (bind _returnvalue (`GameplayStatics.CreateSaveGameObject` "/Game/Project/Menus_y_Widgets/SaveGame_BP.SaveGame_BP_C"))
  (set `/Game/Project/Menus_y_Widgets/SaveGame_BP.SavedScore` (`/Game/ThirdPersonBP/Blueprints/ThirdPersonCharacter.Score` _asthird_person_character) _returnvalue)
  (set `/Game/Project/Menus_y_Widgets/SaveGame_BP.SavedLife` (`/Game/ThirdPersonBP/Blueprints/ThirdPersonCharacter.currentLife` _asthird_person_character) _returnvalue)
  (set `/Game/Project/Menus_y_Widgets/SaveGame_BP.SavedPower` (`/Game/ThirdPersonBP/Blueprints/ThirdPersonCharacter.currentPower` _asthird_person_character) _returnvalue)
  (set `/Game/Project/Menus_y_Widgets/SaveGame_BP.SavedTransform` (`Actor.GetTransform` _asthird_person_character) _returnvalue)
  (`GameplayStatics.SaveGameToSlot` _returnvalue "SavedGame"))

(event `Load`)