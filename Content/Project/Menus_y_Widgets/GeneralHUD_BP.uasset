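; General HUD Blueprint that manages the main menu, pause menu and in-game HUD widgets.
; On BeginPlay it creates all three for player 0, adds them to the viewport and collapses them.
; SetMainMenu, SetInPlay and SetPause switch widget visibility, input mode and mouse cursor, with the latter two also setting game pause.
; SetPause leaves the in-game HUD's visibility untouched, and SetInPlay runs without the re-instantiation check the others have.
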(event `self.ReceiveBeginPlay`
  (`self.InstantiateMenus`))

(event `InstantiateMenus`
  (bind _returnvalue (`GameplayStatics.GetPlayerController` 0))
  (bind _ingamemenu (`self.InGameMenu`))
  (`|ExecutionSequence`
    (:`then_0`
      (bind _returnvalue_2 (`|CreateWidget` "/Game/Project/Menus_y_Widgets/Menu.Menu_C" _returnvalue))
      (bind _output_get (set `self.MainMenu` _returnvalue_2))
      (`UserWidget.AddToViewport` _output_get 0)
      (`Widget.SetVisibility` (`self.MainMenu`) "Collapsed"))
    (:`then_1`
      (bind _returnvalue_3 (`|CreateWidget` "/Game/Project/Menus_y_Widgets/PauseMenu.PauseMenu_C" _returnvalue))
      (bind _output_get_2 (set `self.PauseMenu` _returnvalue_3))
      (`UserWidget.AddToViewport` _output_get_2 0)
      (`Widget.SetVisibility` (`self.PauseMenu`) "Collapsed"))
    (:`then_2`
      (bind _returnvalue_4 (`|CreateWidget` "/Game/Project/Menus_y_Widgets/Widget_HUD.Widget_HUD_C" (`GameplayStatics.GetPlayerController` 0)))
      (set `self.InGameMenu` _returnvalue_4)
      (`UserWidget.AddToViewport` _ingamemenu 0)
      (`Widget.SetVisibility` _ingamemenu "Collapsed"))))

(fn `SetInPlay`
  (bind _returnvalue (`GameplayStatics.GetPlayerController` 0))
  (set `PlayerController.bShowMouseCursor` false _returnvalue)
  (`WidgetBlueprintLibrary.SetInputMode_GameOnly` _returnvalue)
  (`GameplayStatics.SetGamePaused` false)
  (`Widget.SetVisibility` (`self.MainMenu`) "Collapsed")
  (`Widget.SetVisibility` (`self.PauseMenu`) "Collapsed")
  (`Widget.SetVisibility` (`self.InGameMenu`) "Visible"))

(fn `SetMainMenu`
  (bind _returnvalue (`GameplayStatics.GetPlayerController` 0))
  (if (== (`self.MainMenu`) null)
    (`self.InstantiateMenus`))
  (`Widget.SetVisibility` (`self.MainMenu`) "Visible")
  (`WidgetBlueprintLibrary.SetInputMode_UIOnlyEx` _returnvalue (`self.MainMenu`))
  (set `PlayerController.bShowMouseCursor` true _returnvalue)
  (`Widget.SetVisibility` (`self.PauseMenu`) "Collapsed")
  (`Widget.SetVisibility` (`self.InGameMenu`) "Collapsed"))

(fn `SetPause`
  (bind _returnvalue (`GameplayStatics.GetPlayerController` 0))
  (if (== (`self.PauseMenu`) null)
    (`self.InstantiateMenus`))
  (`GameplayStatics.SetGamePaused` true)
  (`Widget.SetVisibility` (`self.PauseMenu`) "Visible")
  (`WidgetBlueprintLibrary.SetInputMode_UIOnlyEx` _returnvalue (`self.PauseMenu`))
  (set `PlayerController.bShowMouseCursor` true _returnvalue)
  (`Widget.SetVisibility` (`self.MainMenu`) "Collapsed"))

(fn `UserConstructionScript`)