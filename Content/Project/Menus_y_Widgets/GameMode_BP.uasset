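; GameMode Blueprint that sets the HUD to match the game's current state when play begins.
; BeginPlay calls OnChangeState, which reads GameState from GameInstance_BP and switches between Main Menu, In Play and Pause Menu.
; Each case calls the matching setup function on the first player's GeneralHUD_BP: SetMainMenu, SetInPlay or SetPause.
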(event `self.ReceiveBeginPlay`
  ;[1 1 1] Situa al empezar el juego en el estado correcto
  (`self.OnChangeState`))

(event `OnChangeState`
  (bind _asgeneral_hud_bp (cast `/Game/Project/Menus_y_Widgets/GeneralHUD_BP` (`PlayerController.GetHUD` (`GameplayStatics.GetPlayerController` 0)) :!pure true))
  (bind _asgame_instance_bp (cast `/Game/Project/Menus_y_Widgets/GameInstance_BP` (`GameplayStatics.GetGameInstance`)))
  (switch `/Game/Project/Menus_y_Widgets/GameStates` (`/Game/Project/Menus_y_Widgets/GameInstance_BP.GameState` _asgame_instance_bp)
    (:`NewEnumerator0`
      (`/Game/Project/Menus_y_Widgets/GeneralHUD_BP.SetMainMenu` _asgeneral_hud_bp))
    (:`NewEnumerator1`
      (`/Game/Project/Menus_y_Widgets/GeneralHUD_BP.SetInPlay` _asgeneral_hud_bp))
    (:`NewEnumerator2`
      (`/Game/Project/Menus_y_Widgets/GeneralHUD_BP.SetPause` _asgeneral_hud_bp))))

(fn `UserConstructionScript`)