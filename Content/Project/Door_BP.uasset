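; Key-locked door that slides along Z for the player and acts as a one-time save checkpoint.
; Front collider overlap by a ThirdPersonCharacter with a key uses it and plays a timeline that adds a local offset every update; leaving stops the timeline.
; Back collider overlap snaps the mesh to its BeginPlay position and saves through GameInstance_BP on the first pass only.
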(event `self.ReceiveBeginPlay`
  (set `self.PosStart` (`SceneComponent.RelativeLocation` (`self.StaticMesh`))))

(event `self.FrontCollider.OnComponentBeginOverlap`
  (params (OverlappedComponent :type "PrimitiveComponent Object Reference") (OtherActor :type "Actor Object Reference") (OtherComp :type "PrimitiveComponent Object Reference") (OtherBodyIndex :type Integer) (bFromSweep :type Boolean) (SweepResult :type "HitResult Structure (by ref)"))
  (bind (_asthird_person_character _bsuccess) (cast `/Game/ThirdPersonBP/Blueprints/ThirdPersonCharacter` OtherActor :!pure true))
  (bind (_posstart_x _posstart_y _posstart_z) (`KismetMathLibrary.BreakVector` (`self.PosStart`)))
  (if _bsuccess
    (if (`/Game/ThirdPersonBP/Blueprints/ThirdPersonCharacter.hasKey` _asthird_person_character)
      (`/Game/ThirdPersonBP/Blueprints/ThirdPersonCharacter.UseKey` _asthird_person_character)
      (bind (_direction _offset) (`Timeline|DoorTL` :!label _label)
        (:`Update`
          (`SceneComponent.K2_AddLocalOffset` (`self.StaticMesh`) (`KismetMathLibrary.MakeVector` 0.0 0.0 (+ _posstart_z (* (`self.MaxOffset`) _offset))) false false))))))

(event `self.FrontCollider.OnComponentEndOverlap`
  (params (OverlappedComponent :type "PrimitiveComponent Object Reference") (OtherActor :type "Actor Object Reference") (OtherComp :type "PrimitiveComponent Object Reference") (OtherBodyIndex :type Integer))
  (if (`.bSuccess` (cast `/Game/ThirdPersonBP/Blueprints/ThirdPersonCharacter` OtherActor :!pure true))
    (goto _label :!via `Stop`)))

(event `CloseDoor`
  (`SceneComponent.K2_SetRelativeLocation` (`self.StaticMesh`) (`self.PosStart`) false false))

(event `self.BackCollider.OnComponentBeginOverlap`
  (params (OverlappedComponent :type "PrimitiveComponent Object Reference") (OtherActor :type "Actor Object Reference") (OtherComp :type "PrimitiveComponent Object Reference") (OtherBodyIndex :type Integer) (bFromSweep :type Boolean) (SweepResult :type "HitResult Structure (by ref)"))
  (if (`.bSuccess` (cast `/Game/ThirdPersonBP/Blueprints/ThirdPersonCharacter` OtherActor :!pure true))
    (`self.CloseDoor`)
    (if (not (`self.hasSaved`))
      (`/Game/Project/MENUS/GameInstance_BP.Save` (cast `/Game/Project/MENUS/GameInstance_BP` (`GameplayStatics.GetGameInstance`) :!pure true))
      (set `self.hasSaved` true))))

(fn `UserConstructionScript`)