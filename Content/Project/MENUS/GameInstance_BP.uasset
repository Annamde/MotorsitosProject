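; Game instance that saves and loads the player's progress through a single fixed save slot.
; Save writes the ThirdPersonCharacter's score, life, power and transform into a new SaveGame_BP object.
; Load checks that the slot exists, restores those values and the transform to the character, then refreshes its life and power bars.
; The Restart event is an empty stub.
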(event `Restart`)

(event `Save`
  (bind _asthird_person_character (cast `/Game/ThirdPersonBP/Blueprints/ThirdPersonCharacter` (`GameplayStatics.GetPlayerPawn` 0) :!pure true))
  (bind _returnvalue (`GameplayStatics.CreateSaveGameObject` "/Game/Project/MENUS/SaveGame_BP.SaveGame_BP_C"))
  (set `/Game/Project/MENUS/SaveGame_BP.SavedScore` (`/Game/ThirdPersonBP/Blueprints/ThirdPersonCharacter.Score` _asthird_person_character) _returnvalue)
  (set `/Game/Project/MENUS/SaveGame_BP.SavedLife` (`/Game/ThirdPersonBP/Blueprints/ThirdPersonCharacter.currentLife` _asthird_person_character) _returnvalue)
  (set `/Game/Project/MENUS/SaveGame_BP.SavedPower` (`/Game/ThirdPersonBP/Blueprints/ThirdPersonCharacter.currentPower` _asthird_person_character) _returnvalue)
  (set `/Game/Project/MENUS/SaveGame_BP.SavedTransform` (`Actor.GetTransform` _asthird_person_character) _returnvalue)
  (`GameplayStatics.SaveGameToSlot` _returnvalue "SavedGame"))

(event `Load`
  (bind _asthird_person_character (cast `/Game/ThirdPersonBP/Blueprints/ThirdPersonCharacter` (`GameplayStatics.GetPlayerPawn` 0) :!pure true))
  (bind _returnvalue (`GameplayStatics.DoesSaveGameExist` "SavedGame"))
  (if _returnvalue
    (bind _returnvalue_2 (`GameplayStatics.LoadGameFromSlot` "SavedGame"))
    (bind _assave_game_bp (cast `/Game/Project/MENUS/SaveGame_BP` _returnvalue_2))
    (set `/Game/ThirdPersonBP/Blueprints/ThirdPersonCharacter.Score` (`/Game/Project/MENUS/SaveGame_BP.SavedScore` _assave_game_bp) _asthird_person_character)
    (set `/Game/ThirdPersonBP/Blueprints/ThirdPersonCharacter.currentLife` (`/Game/Project/MENUS/SaveGame_BP.SavedLife` _assave_game_bp) _asthird_person_character)
    (set `/Game/ThirdPersonBP/Blueprints/ThirdPersonCharacter.currentPower` (`/Game/Project/MENUS/SaveGame_BP.SavedPower` _assave_game_bp) _asthird_person_character)
    (bind _savedtransform (`/Game/Project/MENUS/SaveGame_BP.SavedTransform` _assave_game_bp))
    (`Actor.K2_SetActorTransform` _asthird_person_character _savedtransform false false)
    (`/Game/ThirdPersonBP/Blueprints/ThirdPersonCharacter.UpdateLifeBar` _asthird_person_character)
    (`/Game/ThirdPersonBP/Blueprints/ThirdPersonCharacter.UpdatePowerBar` _asthird_person_character)
    (`Actor.K2_SetActorRotation` _asthird_person_character (`KismetMathLibrary.TransformRotation` _savedtransform) false)))